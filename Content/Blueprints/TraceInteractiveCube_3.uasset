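; Interactive cube that reacts to trace hover and press events with color changes and a timed progress ring.
; Tick yaws and rolls the ring plane toward the player and accumulates hover time once TraceMove flags a hit.
; TraceMove feeds that time into the ring material and aligns an arrow to the surface; after about a second the ring hides and the cube recolors.
; A press halts these TraceMove updates until the trace leaves, which resets everything.
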(event `self.ReceiveBeginPlay`
  (set `self.tiempoestablecido` false)
  (set `self.contador` 0.0)
  (set `self.RayoAlcanzado` false)
  (bind _returnvalue (`KismetMaterialLibrary.CreateDynamicMaterialInstance` "/Game/Materials/UIRing.UIRing" "Ring"))
  (set `self.RingMaterial` _returnvalue)
  (bind _returnvalue_2 (`KismetMaterialLibrary.CreateDynamicMaterialInstance` "/Engine/Functions/Engine_MaterialFunctions02/ExampleContent/3dParticleOpacity_Mat.3dParticleOpacity_Mat"))
  (set `self.DefaultMaterial` _returnvalue_2))

(event `self.ReceiveTick`
  (params (DeltaSeconds :type "Float (single-precision)"))
  (`self.Rotacion`)
  (if (`self.RayoAlcanzado`)
    (`|ExecutionSequence`
      (:`then_0`
        (if (not (`self.tiempoestablecido`))
          (set `self.tiempoestablecido` true)
          (set `self.primer tiempo` DeltaSeconds)))
      (:`then_1`
        (set `self.contador` (+ DeltaSeconds (`self.contador`)))))))

(fn `Rotacion`
  (bind _plane (`self.Plane`))
  (bind (_returnvalue_roll _returnvalue_pitch _returnvalue_yaw) (`KismetMathLibrary.BreakRotator` (`KismetMathLibrary.FindLookAtRotation` (`SceneComponent.K2_GetComponentLocation` _plane) (`SceneComponent.K2_GetComponentLocation` (`Character.Mesh` (`GameplayStatics.GetPlayerCharacter` 0))))))
  (`SceneComponent.K2_SetWorldRotation` _plane (`KismetMathLibrary.MakeRotator` _returnvalue_roll -90.0 _returnvalue_yaw) false false))

(fn `TraceActivateDown`
  (params (Hit :type "HitResult Structure") (Instigator :type "Pawn Object Reference"))
  (returns (Return :type Boolean))
  (`MeshComponent.SetVectorParameterValueOnMaterials` (`self.Cube`) "Color" (0.0 1.0 0.0))
  (`PrimitiveComponent.SetMaterial` (`self.Plane`) 0 (`self.DefaultMaterial`))
  (return false))

(fn `TraceActivateUp`
  (params (Hit :type "HitResult Structure") (Instigator :type "Pawn Object Reference (by ref)"))
  (returns (Return :type Boolean))
  (set `self.botonpulsado` true)
  (`MeshComponent.SetVectorParameterValueOnMaterials` (`self.Cube`) "Color" (1.0 1.0 0.0))
  (return false))

(fn `TraceHitComponent`
  (params (Hit :type "HitResult Structure") (Component :type "PrimitiveComponent Object Reference"))
  (returns (Return :type Boolean))
  (return false))

(fn `TraceHitObject`
  (params (Hit :type "HitResult Structure"))
  (returns (Return :type Boolean))
  (`PrimitiveComponent.SetMaterial` (`self.Plane`) 0 (`self.RingMaterial`))
  (`MeshComponent.SetVectorParameterValueOnMaterials` (`self.Cube`) "Color" (1.0 1.0 0.0))
  (return false))

(fn `TraceLeaveComponent`
  (params (Component :type "PrimitiveComponent Object Reference") (Hit :type "HitResult Structure"))
  (returns (Return :type Boolean))
  (return false))

(fn `TraceLeaveObject`
  (params (Hit :type "HitResult Structure"))
  (returns (Return :type Boolean))
  (`PrimitiveComponent.SetMaterial` (`self.Plane`) 0 (`self.DefaultMaterial`))
  (set `self.primer tiempo` 0.0)
  (set `self.contador` 0.0)
  (set `self.RayoAlcanzado` false)
  (set `self.tiempoestablecido` false)
  (set `self.botonpulsado` false)
  (`MeshComponent.SetVectorParameterValueOnMaterials` (`self.Cube`) "Color" (1.0 1.0 1.0))
  (return false))

(fn `TraceMove`
  (params (Hit :type "HitResult Structure (by ref)"))
  (returns (Return :type Boolean))
  (bind (_bblockinghit _binitialoverlap _time _distance _location _impactpoint _normal) (`GameplayStatics.BreakHitResult` Hit))
  (if (not (`self.botonpulsado`))
    (set `self.RayoAlcanzado` true)
    (`MeshComponent.SetScalarParameterValueOnMaterials` (`self.Plane`) "PercentComplete" (- (`self.contador`) (`self.primer tiempo`)))
    (`SceneComponent.K2_SetWorldLocationAndRotation` (`self.Arrow`) _location (`KismetMathLibrary.Conv_VectorToRotator` _normal) false false)
    (if (> (`self.contador`) 1.0)
      (`PrimitiveComponent.SetMaterial` (`self.Plane`) 0 (`self.DefaultMaterial`))
      (`MeshComponent.SetVectorParameterValueOnMaterials` (`self.Cube`) "Color" (0.7 2.0 1.0))
      (return false))))

(fn `UserConstructionScript`)