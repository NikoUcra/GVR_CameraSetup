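; Interactive cube that responds to trace callbacks with color changes and a dwell-progress ring on its Plane.
; BeginPlay creates ring and default dynamic materials, swapped as the trace enters and leaves.
; Tick increments Contador through a short Delay even without a trace, and only leaving resets it.
; TraceMove feeds Contador to PercentComplete and, past full, hides the ring and recolors the cube; activate down and up only change color.
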(event `self.ReceiveBeginPlay`
  (set `self.Contador` 0.0)
  (bind _returnvalue (`KismetMaterialLibrary.CreateDynamicMaterialInstance` "/Game/Materials/UIRing.UIRing" "Ring"))
  (set `self.RingMaterial` _returnvalue)
  (bind _returnvalue_2 (`KismetMaterialLibrary.CreateDynamicMaterialInstance` "/Engine/Functions/Engine_MaterialFunctions02/ExampleContent/3dParticleOpacity_Mat.3dParticleOpacity_Mat"))
  (set `self.DefaultMaterial` _returnvalue_2))

(event `self.ReceiveTick`
  (params (DeltaSeconds :type "Float (single-precision)"))
  (`KismetSystemLibrary.Delay` 0.01)
  (set `self.Contador` (+ (`self.Contador`) 0.00156)))

(fn `TraceActivateDown`
  (params (Hit :type "HitResult Structure") (Instigator :type "Pawn Object Reference"))
  (returns (Return :type Boolean))
  (`MeshComponent.SetVectorParameterValueOnMaterials` (`self.Cube`) "Color" (0.0 1.0 0.0))
  (return false))

(fn `TraceActivateUp`
  (params (Hit :type "HitResult Structure") (Instigator :type "Pawn Object Reference (by ref)"))
  (returns (Return :type Boolean))
  (`MeshComponent.SetVectorParameterValueOnMaterials` (`self.Cube`) "Color" (1.0 1.0 0.0))
  (return false))

(fn `TraceHitComponent`
  (params (Hit :type "HitResult Structure") (Component :type "PrimitiveComponent Object Reference"))
  (returns (Return :type Boolean))
  (return false))

(fn `TraceHitObject`
  (params (Hit :type "HitResult Structure"))
  (returns (Return :type Boolean))
  (`PrimitiveComponent.SetMaterial` (`self.Plane`) 0 (`self.RingMaterial`))
  (`MeshComponent.SetVectorParameterValueOnMaterials` (`self.Cube`) "Color" (1.0 1.0 0.0))
  (return false))

(fn `TraceLeaveComponent`
  (params (Component :type "PrimitiveComponent Object Reference") (Hit :type "HitResult Structure"))
  (returns (Return :type Boolean))
  (return false))

(fn `TraceLeaveObject`
  (params (Hit :type "HitResult Structure"))
  (returns (Return :type Boolean))
  (`PrimitiveComponent.SetMaterial` (`self.Plane`) 0 (`self.DefaultMaterial`))
  (set `self.Contador` 0.0)
  (`MeshComponent.SetVectorParameterValueOnMaterials` (`self.Cube`) "Color" (1.0 1.0 1.0))
  (return false))

(fn `TraceMove`
  (params (Hit :type "HitResult Structure (by ref)"))
  (returns (Return :type Boolean))
  (`MeshComponent.SetScalarParameterValueOnMaterials` (`self.Plane`) "PercentComplete" (`self.Contador`))
  (if (> (`self.Contador`) 1.0)
    (`PrimitiveComponent.SetMaterial` (`self.Plane`) 0 (`self.DefaultMaterial`))
    (`MeshComponent.SetVectorParameterValueOnMaterials` (`self.Cube`) "Color" (0.7 2.0 1.0))
    (return false)))

(fn `UserConstructionScript`)